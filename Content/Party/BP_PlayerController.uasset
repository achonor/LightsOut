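; Player controller for the Party game that applies the player's chosen type to the pawn they control.
; On BeginPlay, the local controller reads PlayerType from BP_GameInstance through a getter that caches the cast reference.
; When the type changes, SetPlayerType stores it, destroys any controlled pawn and has the GameMode restart the player to respawn them.
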(event `self.ReceiveBeginPlay`
  (if (`self.IsLocalController`)
    (bind _gameinstanceref (`self.GetGameInstance`))
    (`self.SetPlayerType` (`/Game/Party/BP_GameInstance.PlayerType` _gameinstanceref))))

(event `SetPlayerType`
  (params (PlayerType :type "/Game/Party/Blueprints/Public/Enum/E_PlayerType Enum" :default "NewEnumerator0"))
  (bind _returnvalue (`self.K2_GetPawn`))
  (if (`|EnumInequality` PlayerType (`self.PlayerType`))
    (set `self.PlayerType` PlayerType)
    (`/Engine/EditorBlueprintResources/StandardMacros.IsValid` _returnvalue
      (:`Is Valid`
        (`self.K2_DestroyActor` _returnvalue))
      (:`Is Not Valid`
        _))
    (`GameModeBase.RestartPlayer` (`GameplayStatics.GetGameMode`) self)))

(fn `GetGameInstance`
  (returns (GameInstanceRef :type "/Game/Party/BP_GameInstance Object Reference"))
  (bind _gameinstanceref (`self.GameInstanceRef`))
  (`/Engine/EditorBlueprintResources/StandardMacros.IsValid` _gameinstanceref
    (:`Is Valid`
      (return _gameinstanceref))
    (:`Is Not Valid`
      (bind _asbp_game_instance (cast `/Game/Party/BP_GameInstance` (`GameplayStatics.GetGameInstance`)))
      (bind _output_get (set `self.GameInstanceRef` _asbp_game_instance))
      (return _output_get))))

(fn `UserConstructionScript`)