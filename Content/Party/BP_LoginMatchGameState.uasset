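; Game state for the login/matchmaking lobby that tracks human and monster slot counts and launches the match.
; Request and cancel functions adjust the current counts against per-side maximums; their RepNotifies refresh every top-level UI_Match widget after a short delay.
; StartGame, on authority only, gives each BP_LoginMatchPlayerController a sequential index within its side, then server-travels to DefaultMap after a brief delay.
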(event `StartGame`
  (bind _temphumancnt (`self.TempHumanCnt`))
  (bind _tempmonstercnt (`self.TempMonsterCnt`))
  (`/Engine/EditorBlueprintResources/ActorMacros.Switch Has Authority`
    (:`Authority`
      (`|ExecutionSequence`
        (:`then_0`
          (set `self.TempHumanCnt` 0)
          (set `self.TempMonsterCnt` 0))
        (:`then_1`
          (bind _outactors (`GameplayStatics.GetAllActorsOfClass` "/Game/Party/BP_LoginMatchPlayerController.BP_LoginMatchPlayerController_C"))
          (for _array_element _outactors
            (if (`/Game/Party/BP_LoginMatchPlayerController.IsHuman` _array_element)
              (`/Game/Party/BP_LoginMatchPlayerController.SetPlayerIndex` _array_element _temphumancnt)
              (set `self.TempHumanCnt` (+ _temphumancnt 1))
              (else
                (`/Game/Party/BP_LoginMatchPlayerController.SetPlayerIndex` _array_element _tempmonstercnt)
                (set `self.TempMonsterCnt` (+ _tempmonstercnt 1))))))
        (:`then_2`
          (`KismetSystemLibrary.Delay` 0.2)
          (`KismetSystemLibrary.ExecuteConsoleCommand` "servertravel DefaultMap" null))))))

(event `RefreshMatchUI`
  (`KismetSystemLibrary.Delay` 0.2)
  (bind _foundwidgets (`WidgetBlueprintLibrary.GetAllWidgetsOfClass` "/Game/Party/UI/UI_Match.UI_Match_C"))
  (for _array_element _foundwidgets
    (`/Game/Party/UI/UI_Match.RefreshUI` _array_element)))

(fn `CancelHuman`
  (set `self.CurHumanCount` (+ (`self.CurHumanCount`) -1)))

(fn `CancelMonster`
  (set `self.CurMonsterCount` (+ (`self.CurMonsterCount`) -1)))

(fn `GetLastHumanCount`
  (returns (Count :type Integer))
  (return (- (`self.HumanCountMax`) (`self.CurHumanCount`))))

(fn `GetLastMonsterCount`
  (returns (Count :type Integer))
  (return (- (`self.MonsterCountMax`) (`self.CurMonsterCount`))))

(fn `OnRep_CurHumanCount`
  (`self.RefreshMatchUI`))

(fn `OnRep_CurMonsterCount`
  (`self.RefreshMatchUI`))

(fn `RequestHuman`
  (returns (result :type Boolean))
  (bind _count (`self.GetLastHumanCount`))
  (if (>= _count 1)
    (set `self.CurHumanCount` (+ (`self.CurHumanCount`) 1))
    (return true)
    (else
      (return false))))

(fn `RequestMonster`
  (returns (result :type Boolean))
  (bind _count (`self.GetLastMonsterCount`))
  (if (>= _count 1)
    (set `self.CurMonsterCount` (+ (`self.CurMonsterCount`) 1))
    (return true)
    (else
      (return false))))

(fn `UserConstructionScript`)