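; Game state for a human-versus-monster match that runs the countdown, decides the result and returns to WaitMap.
; Tick drives the countdown into CheckGameOver, which picks a result from time left and the states of human and monster actors.
; OnGameOver shows the result widget before a delayed server travel, while a looping timer refreshes the game UI countdown.
; The server fills player-indexed human and monster arrays, retrying until every index is assigned.
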(event `OnGameOver`
  (params (Result :type "/Game/Party/Blueprints/Public/Enum/E_GameResult Enum" :default "NewEnumerator0"))
  (bind _returnvalue (`|CreateWidget` "/Game/Party/UI/UI_GameOver.UI_GameOver_C"))
  (`UserWidget.AddToViewport` _returnvalue 0)
  (`/Game/Party/UI/UI_GameOver.Set Game Result` _returnvalue Result)
  (`KismetSystemLibrary.Delay` 5.0)
  (`KismetSystemLibrary.ExecuteConsoleCommand` "servertravel WaitMap" null))

(event `CheckGameOver`
  (if (<= (`self.GameCountdown`) 0.0)
    (`self.OnGameOver` "NewEnumerator2")
    (else
      (`|ExecutionSequence`
        (:`then_0`
          (set `self.HasHuman` false)
          (set `self.HasMonster` false))
        (:`then_1`
          (bind _outactors (`GameplayStatics.GetAllActorsOfClass` "/Game/Party/Blueprints/BP_Human.BP_Human_C"))
          (for _array_element _outactors
            (if (`|EnumInequality` (`/Game/Party/Blueprints/BP_Human.player_state_current` _array_element) "NewEnumerator2")
              (set `self.HasHuman` true)
              (break))))
        (:`then_2`
          (bind _outactors_2 (`GameplayStatics.GetAllActorsOfClass` "/Game/Party/Blueprints/BP_Monster.BP_Monster_C"))
          (for _array_element_2 _outactors_2
            (if (`|EnumInequality` (`/Game/Party/Blueprints/BP_Monster.player_state_current` _array_element_2) "NewEnumerator2")
              (set `self.HasMonster` true)
              (break))))
        (:`then_3`
          (if (`self.HasHuman`)
            (if (`self.HasMonster`)
              (`self.OnGameOver` "NewEnumerator0"))
            (else
              (`self.OnGameOver` "NewEnumerator1"))))))))

(event `self.ReceiveTick`
  (params (DeltaSeconds :type "Float (single-precision)"))
  (bind _output_get (set `self.GameCountdown` (- (`self.GameCountdown`) DeltaSeconds)))
  (if (<= _output_get 0.0)
    (`self.CheckGameOver`)))

(event `self.ReceiveBeginPlay`
  (`KismetSystemLibrary.K2_SetTimerDelegate` (delegate `RefreshCountdown`) 1.0 true)
  (`self.CollectHumanAndMonster`))

(event `RefreshCountdown`
  (bind _uigame (`self.GetGameUI`))
  (`/Engine/EditorBlueprintResources/StandardMacros.IsValid` _uigame
    (:`Is Valid`
      (`/Game/Party/UI/UI_Game.RefreshCountdown` _uigame (`self.GameCountdown`)))))

(event `CollectHumanAndMonster`
  ;[1 1 1] 收集人数组，鬼数组
  (`/Engine/EditorBlueprintResources/ActorMacros.Switch Has Authority`
    (:`Authority`
      (`KismetSystemLibrary.Delay` 1.0)
      (`|ExecutionSequence`
        (:`then_0`
          (`KismetArrayLibrary.Array_Clear` (`self.HumanList`))
          (`KismetArrayLibrary.Array_Clear` (`self.MonsterList`))
          (set `self.CollectFinished` true))
        (:`then_1`
          (bind _outactors (`GameplayStatics.GetAllActorsOfClass` "/Game/Party/Blueprints/BP_Human.BP_Human_C"))
          (for _array_element _outactors
            (bind _player_index (`/Game/Party/Blueprints/BP_Human.player_index` _array_element))
            (if (!= _player_index -1)
              (`KismetArrayLibrary.Array_Set` (`self.HumanList`) _player_index _array_element true)
              (else
                (set `self.CollectFinished` false)))))
        (:`then_2`
          (bind _outactors_2 (`GameplayStatics.GetAllActorsOfClass` "/Game/Party/Blueprints/BP_Monster.BP_Monster_C"))
          (for _array_element_2 _outactors_2
            (bind _player_index_2 (`/Game/Party/Blueprints/BP_Monster.player_index` _array_element_2))
            (if (!= _player_index_2 -1)
              (`KismetArrayLibrary.Array_Set` (`self.MonsterList`) _player_index_2 _array_element_2 true)
              (else
                (set `self.CollectFinished` false)))))
        (:`then_3`
          ;;[1 1 1] 有客户端还没提交，重新收集
          (if (not (`self.CollectFinished`))
            (`self.CollectHumanAndMonster`)))))))

(fn `GetGameUI`
  (returns (UIGame :type "/Game/Party/UI/UI_Game Object Reference"))
  (bind _uigameinstance (`self.UIGameInstance`))
  (`/Engine/EditorBlueprintResources/StandardMacros.IsValid` _uigameinstance
    (:`Is Valid`
      (return _uigameinstance))
    (:`Is Not Valid`
      (bind _foundwidgets (`WidgetBlueprintLibrary.GetAllWidgetsOfClass` "/Game/Party/UI/UI_Game.UI_Game_C"))
      (bind _output_get (set `self.UIGameInstance` (`|GetArrayItem` _foundwidgets)))
      (return _output_get))))

(fn `GetMonsterByIndex`
  (params (Index :type Integer))
  (returns (Monster :type "/Game/Party/Blueprints/BP_Monster Object Reference"))
  (return (`|GetArrayItem` (`self.MonsterList`) Index)))

(fn `UserConstructionScript`)