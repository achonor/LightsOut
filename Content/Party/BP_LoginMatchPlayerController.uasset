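; Player controller for the login and matchmaking stage that handles choosing the Human or Monster role and starting the game.
; Each selection releases any previous pick, then requests the role from BP_LoginMatchGameState, which it caches on first lookup.
; An accepted request updates the local selection flags and stores the player type in BP_GameInstance.
; A separate event stores the player index in the same game instance, and StartGame forwards to the game state.
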(event `StartGame`
  (bind _gamestate (`self.GetGameState`))
  (`/Game/Party/BP_LoginMatchGameState.StartGame` _gamestate))

(event `SelectHuman`
  (bind _gamestate (`self.GetGameState`))
  (`self.CancelSelect`)
  (bind _result (`/Game/Party/BP_LoginMatchGameState.RequestHuman` _gamestate))
  (if _result
    (`self.SetPlayerType` true)
    (set `self.IsSelected` true)
    (set `self.IsHuman` true)))

(event `SelectMonster`
  (bind _gamestate (`self.GetGameState`))
  (`self.CancelSelect`)
  (bind _result (`/Game/Party/BP_LoginMatchGameState.RequestMonster` _gamestate))
  (if _result
    (`self.SetPlayerType` false)
    (set `self.IsSelected` true)
    (set `self.IsHuman` false)))

(event `CancelSelect`
  (if (`self.IsSelected`)
    (bind _gamestate (`self.GetGameState`))
    (if (`self.IsHuman`)
      (`/Game/Party/BP_LoginMatchGameState.CancelHuman` _gamestate)
      (else
        (`/Game/Party/BP_LoginMatchGameState.CancelMonster` _gamestate)))
    (set `self.IsSelected` false)
    (set `self.IsHuman` false)))

(event `SetPlayerType`
  (params (IsHuman :type Boolean))
  (bind _asbp_game_instance (cast `/Game/Party/BP_GameInstance` (`GameplayStatics.GetGameInstance`)))
  (if IsHuman
    (set `/Game/Party/BP_GameInstance.PlayerType` "NewEnumerator0" _asbp_game_instance)
    (else
      (set `/Game/Party/BP_GameInstance.PlayerType` "NewEnumerator1" _asbp_game_instance))))

(event `SetPlayerIndex`
  (params (Index :type Integer))
  (bind _asbp_game_instance (cast `/Game/Party/BP_GameInstance` (`GameplayStatics.GetGameInstance`)))
  (set `/Game/Party/BP_GameInstance.PlayerIndex` Index _asbp_game_instance))

(fn `GetGameState`
  (returns (GameState :type "/Game/Party/BP_LoginMatchGameState Object Reference"))
  (bind _gamestateinstance (`self.GameStateInstance`))
  (`/Engine/EditorBlueprintResources/StandardMacros.IsValid` _gamestateinstance
    (:`Is Valid`
      (return _gamestateinstance))
    (:`Is Not Valid`
      (bind _asbp_login_match_game_state (cast `/Game/Party/BP_LoginMatchGameState` (`GameplayStatics.GetGameState`)))
      (bind _output_get (set `self.GameStateInstance` _asbp_login_match_game_state))
      (return _output_get))))

(fn `UserConstructionScript`)