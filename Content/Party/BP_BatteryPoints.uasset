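; BP_BatteryPoints holds red and blue point sets for a party mode, apparently for batteries, and hands out a random point on request.
; GetRandomPoints picks RedPoints for the first enum value of Type and BluePoints for any other, then passes that array to GetRandValue.
; GetRandValue returns a uniformly random element with no empty-array check; the event graph and construction script do nothing.
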(fn `GetRandomPoints`
  (params (Type :type "/Game/Party/Blueprints/Public/Enum/E_BatteryAndLightType Enum" :default "NewEnumerator0"))
  (returns (Point :type "Vector Structure"))
  (if (`|EnumEquality` Type "NewEnumerator0")
    (bind _value (`self.GetRandValue` (`self.RedPoints`)))
    (return _value)
    (else
      (bind _value_2 (`self.GetRandValue` (`self.BluePoints`)))
      (return _value_2))))

(fn `GetRandValue`
  (params (Array :type "Array of Vector Structure"))
  (returns (Value :type "Vector Structure"))
  (return (`|GetArrayItem` Array (`KismetMathLibrary.RandomIntegerInRange` 0 (- (`KismetArrayLibrary.Array_Length` Array) 1)))))

(fn `UserConstructionScript`)