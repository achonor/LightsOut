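; BP_Room is a room actor that can be unlit, have a sabotaged breaker, or be fully lit.
; The RoomState OnRep swaps floor visuals, updates lights, charging cube and fixing cube (breaker) found by room Id, and spawns lightning when fully lit.
; A breaker countdown runs on an authority-only one-second timer, updates a 3D widget, then hides it and destroys the stored fixing cube at expiry.
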(event `设置房间外观`
  (params (isActive :type Boolean))
  ;[1 1 1] 设置房间外观
  (`SceneComponent.SetVisibility` (`self.RoomFloor(未点亮状态)`) (not isActive) false)
  (`SceneComponent.SetVisibility` (`self.RoomFloor(点亮状态)`) isActive false))

(event `修改房间所有灯的状态`
  (params (State :type "/Game/Party/Blueprints/Public/Enum/E_LightState Enum" :default "NewEnumerator0"))
  ;[1 1 1] 改变房间的灯的状态
  (bind _outactors (`GameplayStatics.GetAllActorsOfClass` "/Game/Party/Blueprints/BP_Light.BP_Light_C"))
  (for _array_element _outactors
    (if (== (`/Game/Party/Blueprints/BP_Light.owningRoom` _array_element) (`self.id`))
      (set `/Game/Party/Blueprints/BP_Light.lightState_current` State _array_element))))

(event `修改房间中充电桩的状态`
  (params (`是否可用` :type Boolean))
  ;[1 1 1] 修改房间中充电桩的状态
  (bind _outactors (`GameplayStatics.GetAllActorsOfClass` "/Game/Party/Blueprints/BP_ChargingCube.BP_ChargingCube_C"))
  (for _array_element _outactors
    (if (== (`/Game/Party/Blueprints/BP_ChargingCube.owningRoom` _array_element) (`self.id`))
      (set `/Game/Party/Blueprints/BP_ChargingCube.isUsable?` `是否可用` _array_element)
      (break))))

(event `修改房间中电闸的状态`
  (params (`电闸状态` :type "/Game/Party/Blueprints/Public/Enum/E_FixingCubeState Enum" :default "NewEnumerator0"))
  ;[1 1 1] 修改房间中电闸的状态
  (bind _outactors (`GameplayStatics.GetAllActorsOfClass` "/Game/Party/Blueprints/BP_FixingCube.BP_FixingCube_C"))
  (for _array_element _outactors
    (if (== (`/Game/Party/Blueprints/BP_FixingCube.room_id` _array_element) (`self.id`))
      (`/Game/Party/Blueprints/BP_FixingCube.设置电闸外观` _array_element `电闸状态`)
      (break))))

(event `销毁电闸`
  (bind _fixingcubeobject (`self.fixingCubeObject`))
  ;[1 1 1] 让FixingCube销毁自己
  (`/Engine/EditorBlueprintResources/StandardMacros.IsValid` _fixingcubeobject
    (:`Is Valid`
      (`/Game/Party/Blueprints/BP_FixingCube.销毁自己` _fixingcubeobject))))

(event `开始房间倒计时`
  (params (FixingCube :type "/Game/Party/Blueprints/BP_FixingCube Object Reference"))
  ;[1 1 1] 倒计时相关
  ;;[1 1 1] 开始
  (set `self.fixingCubeObject` FixingCube)
  ;;;[1 1 1] 重置倒计时
  (set `self.countdown_rest` (`self.countdown_max`))
  (`SceneComponent.SetVisibility` (`self.3DUI`) true false)
  (`/Engine/EditorBlueprintResources/ActorMacros.Switch Has Authority`
    (:`Authority`
      (`KismetSystemLibrary.K2_SetTimer` null "持续减少倒计时" 1.0 true)
      ;;;[1 1 1] 显示提示文本
      (bind _as3dui_room (cast `/Game/Party/UI/3DUI_Room` (`WidgetComponent.GetUserWidgetObject` (`self.3DUI`))))
      (set `/Game/Party/UI/3DUI_Room.text_hint` "房间电闸已被破坏" _as3dui_room))))

(event `持续减少倒计时`
  ;[1 1 1] 倒计时相关
  ;;[1 1 1] 持续减少倒计时
  (bind _output_get (set `self.countdown_rest` (- (`self.countdown_rest`) 1)))
  (if (>= _output_get 0)
    ;;;[1 1 1] 倒计时大于0则更新ui
    (bind _as3dui_room (cast `/Game/Party/UI/3DUI_Room` (`WidgetComponent.GetUserWidgetObject` (`self.3DUI`))))
    (set `/Game/Party/UI/3DUI_Room.text_countdown` (`self.countdown_rest`) _as3dui_room)
    (set `/Game/Party/UI/3DUI_Room.text_hint` "" _as3dui_room)
    (else
      (`self.结束倒计时`))))

(event `结束倒计时`
  ;[1 1 1] 倒计时相关
  ;;[1 1 1] 结束倒计时
  (`KismetSystemLibrary.K2_ClearTimer` null "持续减少倒计时")
  (`SceneComponent.SetVisibility` (`self.3DUI`) false false)
  (`self.销毁电闸`))

(fn `OnRep_roomState_current`
  (switch `/Game/Party/Blueprints/Public/Enum/E_RoomState` (`self.roomState_current`)
    (:`NewEnumerator0`
      (`self.设置房间外观` false))
    (:`NewEnumerator1`
      (`self.设置房间外观` false)
      (`self.修改房间所有灯的状态` "NewEnumerator2")
      (`self.修改房间中充电桩的状态` false)
      (`self.修改房间中电闸的状态` "NewEnumerator2"))
    (:`NewEnumerator2`
      (`self.设置房间外观` true)
      (`self.修改房间所有灯的状态` "NewEnumerator1")
      (`self.修改房间中充电桩的状态` true)
      (`self.修改房间中电闸的状态` "NewEnumerator1")
      (`NiagaraFunctionLibrary.SpawnSystemAtLocation` "/Game/Party/Source/VFX/Vefects/Anime_VFX/Shared/Skills/NS_Lightning_Cast.NS_Lightning_Cast" (`self.K2_GetActorLocation`)))))

(fn `UserConstructionScript`)