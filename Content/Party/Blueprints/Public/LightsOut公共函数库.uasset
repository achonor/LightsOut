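; Public function library for the LightsOut party game, with one check for whether an actor falls within a target human's flashlight range.
; The human's current flashlight power, rounded up, indexes distance and angle limit arrays, so reach and cone depend on power.
; Distance is measured from the flashlight component, while the angle uses a dot product and acos against the human actor's forward vector.
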(fn `是否满足距离和角度检测`
  (params (Actor :type "Actor Object Reference") (`目标人类` :type "/Game/Party/Blueprints/BP_Human Object Reference"))
  (returns (`是否满足` :type Boolean))
  (locals (distance :type "Array of Float (double-precision)"))
  (return (and (<= (`KismetMathLibrary.Vector_Distance` (`Actor.K2_GetActorLocation` Actor) (`SceneComponent.K2_GetComponentLocation` (`/Game/Party/Blueprints/BP_Human.Flashlight` `目标人类`))) (`|GetArrayItem` (`local.distance`) (`KismetMathLibrary.Conv_Int64ToInt` (`KismetMathLibrary.FCeil64` (`/Game/Party/Blueprints/BP_Human.flashlight_power_current` `目标人类`))))) (<= (`KismetMathLibrary.DegAcos` (`KismetMathLibrary.Dot_VectorVector` (`KismetMathLibrary.Normal` (- (`Actor.K2_GetActorLocation` Actor) (`Actor.K2_GetActorLocation` `目标人类`))) (`KismetMathLibrary.Normal` (`Actor.GetActorForwardVector` `目标人类`)))) (`|GetArrayItem` (`/Game/Party/Blueprints/BP_Human.flashlight_degree` `目标人类`) (`KismetMathLibrary.Conv_Int64ToInt` (`KismetMathLibrary.FCeil64` (`/Game/Party/Blueprints/BP_Human.flashlight_power_current` `目标人类`))))))))