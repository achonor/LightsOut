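; BP_FixingCube is a room-linked object that a Monster can sabotage and a Human can repair.
; GetRoom finds the BP_Room with a matching RoomId and caches it.
; Sabotage (破坏) and repair (修理) toggle that room's state between two enum values, recording who acted, and repair destroys the cube.
; Events that clear those users are commented as unused, and the overlap events are empty.
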(event `self.StaticMesh.OnComponentBeginOverlap`
  (params (OverlappedComponent :type "PrimitiveComponent Object Reference") (OtherActor :type "Actor Object Reference") (OtherComp :type "PrimitiveComponent Object Reference") (OtherBodyIndex :type Integer) (bFromSweep :type Boolean) (SweepResult :type "HitResult Structure (by ref)")))

(event `self.StaticMesh.OnComponentEndOverlap`
  (params (OverlappedComponent :type "PrimitiveComponent Object Reference") (OtherActor :type "Actor Object Reference") (OtherComp :type "PrimitiveComponent Object Reference") (OtherBodyIndex :type Integer)))

(event `破坏`
  (params (Monster :type "/Game/Party/Blueprints/BP_Monster Object Reference"))
  (bind _room (`self.GetRoom`))
  (if (`|EnumEquality` (`/Game/Party/Blueprints/BP_Room.roomState_current` _room) "NewEnumerator2")
    (set `self.using_monster` Monster)
    (set `/Game/Party/Blueprints/BP_Room.roomState_current` "NewEnumerator1" _room)))

(event `修理`
  (params (Human :type "/Game/Party/Blueprints/BP_Human Object Reference"))
  (bind _room (`self.GetRoom`))
  (if (`|EnumEquality` (`/Game/Party/Blueprints/BP_Room.roomState_current` _room) "NewEnumerator1")
    (`KismetArrayLibrary.Array_Add` (`self.using_humans`) Human)
    (set `/Game/Party/Blueprints/BP_Room.roomState_current` "NewEnumerator2" _room)
    (`self.K2_DestroyActor`)))

(event `结束破坏`
  ;[1 1 1] 结束破坏，暂时没用上，要用自己写
  (set `self.using_monster` null))

(event `退出修理`
  (params (Human :type "/Game/Party/Blueprints/BP_Human Object Reference"))
  ;[1 1 1] 玩家退出修理，暂时没用上，要用自己写
  (`KismetArrayLibrary.Array_RemoveItem` (`self.using_humans`) Human))

(fn `GetRoom`
  (returns (Room :type "/Game/Party/Blueprints/BP_Room Object Reference"))
  (bind _room_object (`self.room_object`))
  (`/Engine/EditorBlueprintResources/StandardMacros.IsValid` _room_object
    (:`Is Valid`
      (return _room_object))
    (:`Is Not Valid`
      (bind _outactors (`GameplayStatics.GetAllActorsOfClass` "/Game/Party/Blueprints/BP_Room.BP_Room_C"))
      (for _array_element _outactors
        (if (== (`/Game/Party/Blueprints/BP_Room.id` _array_element) (`self.room_id`))
          (bind _output_get (set `self.room_object` _array_element))
          (return _output_get))))))

(fn `UserConstructionScript`)